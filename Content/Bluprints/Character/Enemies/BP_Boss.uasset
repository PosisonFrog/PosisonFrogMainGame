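; BP_Boss is a boss enemy character Blueprint with a BossPhaseComponent, and its logic is currently inactive.
; The component's OnPatternStarted event is bound but empty.
; A disconnected three-case switch would play a montage, wait briefly, then AIMoveTo the player pawn.
; Only the first case has a montage assigned, a Donkey skill animation.
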(event OnPatternStarted(BossPhaseComponent)
  (params (PhaseIndex :type Integer) (PatternId :type Name :default "None") (PatternData :type Boss%20Pattern%20Definition%20Structure%20%28by%20ref%29) (RemainingPower :type Float%20%28single-precision%29)))

(event EventBeginPlay)

(event Collision|EventActorBeginOverlap
  (params (OtherActor :type Actor%20Object%20Reference)))

(event EventTick
  (params (DeltaSeconds :type Float%20%28single-precision%29)))

(fn ConstructionScript)